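; Player-controlled rolling ball that restarts the level when it takes damage.
; The MoveForwardBack and MoveLeftRight axes feed a shared AddTorque node on the Sphere, scaled by StrMultiply and applied as an acceleration change.
; BeginPlay fades the camera in, while AnyDamage fades it out, waits for the fade to finish, then reopens the current level by name.
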(event Game|Damage|EventAnyDamage
  (params (Damage :type Float%20%28single-precision%29) (DamageType :type Damage%20Type%20Object%20Reference) (InstigatedBy :type Controller%20Object%20Reference) (DamageCauser :type Actor%20Object%20Reference))
  (CameraFades|StartCameraFade :self (Game|GetPlayerCameraManager 0) :ToAlpha 1.0 :Duration 2.0 :bHoldWhenFinished true)
  (Utilities|FlowControl|Delay 2.1)
  (bind _returnvalue (Game|GetCurrentLevelName true))
  (Game|OpenLevel(byName) (Utilities|String|StringToName _returnvalue)))

(event EventBeginPlay
  (CameraFades|StartCameraFade :self (Game|GetPlayerCameraManager 0) :FromAlpha 1.0 :Duration 2.0 :bHoldWhenFinished true))

(event Input|AxisEvents|InputAxisMoveForwardBack
  (params (AxisValue :type Float%20%28single-precision%29))
  (bind _strmultiply (Variables|BallProperties|GetStrMultiply))
  (Class|PrimitiveComponent|AddTorqueinRadians (Variables|Default|GetSphere) (Math|Vector|MakeVector (* (stale Input|AxisEvents|InputAxisMoveLeftRight AxisValue) _strmultiply) (* AxisValue _strmultiply) 0.0) "None" true))

(event Input|AxisEvents|InputAxisMoveLeftRight
  (params (AxisValue :type Float%20%28single-precision%29))
  (bind _strmultiply (Variables|BallProperties|GetStrMultiply))
  (Class|PrimitiveComponent|AddTorqueinRadians (Variables|Default|GetSphere) (Math|Vector|MakeVector (* AxisValue _strmultiply) (* (stale Input|AxisEvents|InputAxisMoveForwardBack AxisValue) _strmultiply) 0.0) "None" true))

(fn ConstructionScript)