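; BP_Win is a level exit trigger that completes the level when the player enters its box with every crystal collected.
; If any BP_Crystal_01 or BP_Crystal_02 actors remain, it prints a warning; otherwise it fades the camera out and, after a delay, calls CompleteLevel.
; CompleteLevel opens the next entry in the TabLevelNames01 array, or prints "THE END" on the last level.
; BeginPlay fades the camera in from black.
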(event OnComponentBeginOverlap(Box)
  (params (OverlappedComponent :type Primitive%20Component%20Object%20Reference) (OtherActor :type Actor%20Object%20Reference) (OtherComp :type Primitive%20Component%20Object%20Reference) (OtherBodyIndex :type Integer) (bFromSweep :type Boolean) (SweepResult :type Hit%20Result%20Structure%20%28by%20ref%29))
  (Utilities|IsPlayer OtherActor
    (:true
      (bind _outactors (Actor|GetAllActorsOfClass "/Game/Blueprints/BP_Crystal_01.BP_Crystal_01_C"))
      (bind _outactors_2 (Actor|GetAllActorsOfClass "/Game/Blueprints/BP_Crystal_02.BP_Crystal_02_C"))
      (if (or (> (Utilities|Array|Length _outactors_2) 0) (> (Utilities|Array|Length _outactors) 0))
        (Development|PrintString "NIE ZEBRANO WSZYSTKICH KRYSZTALOW")
        (else
          (CameraFades|StartCameraFade :self (Game|GetPlayerCameraManager 0) :ToAlpha 1.0 :Duration 2.0 :bHoldWhenFinished true)
          (Utilities|FlowControl|Delay 2.1)
          (CallFunction|CompleteLevel))))))

(event EventBeginPlay
  (CameraFades|StartCameraFade :self (Game|GetPlayerCameraManager 0) :FromAlpha 1.0 :Duration 2.0 :bHoldWhenFinished true))

(fn ConstructionScript)

(fn GetCurrentLevelIndex
  (bind _returnvalue (Game|GetCurrentLevelName true))
  (return (Utilities|Array|FindItem (Variables|Default|Gettab_LevelNames_01) _returnvalue)))

(fn GetNextLevelName
  (bind _levelindex (CallFunction|GetCurrentLevelIndex))
  (return (Utilities|Array|Get(acopy) (Variables|Default|Gettab_LevelNames_01) (+ _levelindex 1))))

(fn LoadNextLevel
  (bind _output (CallFunction|GetNextLevelName))
  (Game|OpenLevel(byName) (Utilities|String|StringToName _output)))

(fn IsFinalLevel
  (bind _levelindex (CallFunction|GetCurrentLevelIndex))
  (return (== (Utilities|Array|LastIndex (Variables|Default|Gettab_LevelNames_01)) _levelindex)))

(fn CompleteLevel
  (bind _returnvalue (CallFunction|IsFinalLevel))
  (if _returnvalue
    (Development|PrintString "THE END")
    (else
      (CallFunction|LoadNextLevel))))