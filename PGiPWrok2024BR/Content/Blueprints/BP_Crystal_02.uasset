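; BP_Crystal_02 is a crystal pickup that flies to the player and vanishes when the player touches it.
; An overlap on its sphere passes a player check, stores the point light's intensity and plays a timeline.
; Each update lerps the actor from its current transform toward the player pawn's location and zero scale, so the motion follows a moving player.
; The actor destroys itself when the timeline finishes.
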(event OnComponentBeginOverlap(Sphere)
  (params (OverlappedComponent :type Primitive%20Component%20Object%20Reference) (OtherActor :type Actor%20Object%20Reference) (OtherComp :type Primitive%20Component%20Object%20Reference) (OtherBodyIndex :type Integer) (bFromSweep :type Boolean) (SweepResult :type Hit%20Result%20Structure%20%28by%20ref%29))
  (Utilities|IsPlayer OtherActor
    (:true
      (Variables|Default|SetIntensity (Variables|/Script/Engine.LightComponentBase|GetIntensity (Variables|Default|GetPointLight)))
      (bind (_direction _transform_location _transform_scale) (Timeline|Crystal_Transforma_02 Play)
        (:Update
          (Transformation|SetActorLocation (Math|Vector|Lerp(Vector) (Transformation|GetActorLocation) (Transformation|GetActorLocation (Game|Player|GetPlayerPawn 0)) _transform_location) false false)
          (Transformation|SetActorScale3D (Math|Vector|Lerp(Vector) (Transformation|GetActorScale3D) "0, 0, 0" _transform_scale)))
        (:Finished
          (Actor|DestroyActor))))))

(fn ConstructionScript)