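; BP_TiltingPlatform is a platform that tilts while a BP_Ball_01 is inside its trigger zone and levels out afterwards.
; TriggerZone begin and end overlaps check the other actor's class and toggle the IsTilting flag.
; Each Tick, FInterpTo eases PlatformMesh's relative roll toward TiltAngle or back to zero, using TiltSpeed and scaled delta time, with pitch and yaw held at zero.
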(event OnComponentBeginOverlap(TriggerZone)
  (params (OverlappedComponent :type Primitive%20Component%20Object%20Reference) (OtherActor :type Actor%20Object%20Reference) (OtherComp :type Primitive%20Component%20Object%20Reference) (OtherBodyIndex :type Integer) (bFromSweep :type Boolean) (SweepResult :type Hit%20Result%20Structure%20%28by%20ref%29))
  ;[1 0.2625 0.3925] Event overlap for TriggerZone
  (bind _asbp_ball_01 (Utilities|Casting|CastToBP_Ball_01Class (Utilities|GetClass OtherActor)))
  (Variables|Default|SetIsTilting true))

(event OnComponentEndOverlap(TriggerZone)
  (params (OverlappedComponent :type Primitive%20Component%20Object%20Reference) (OtherActor :type Actor%20Object%20Reference) (OtherComp :type Primitive%20Component%20Object%20Reference) (OtherBodyIndex :type Integer))
  ;[1 0.2625 0.3925] Event overlap for TriggerZone
  (bind _asbp_ball_01 (Utilities|Casting|CastToBP_Ball_01Class (Utilities|GetClass OtherActor)))
  (Variables|Default|SetIsTilting false))

(event EventTick
  (params (DeltaSeconds :type Float%20%28single-precision%29))
  (bind _deltamultiplier (Variables|Default|GetDeltaMultiplier))
  (bind _platformmesh (Variables|Default|GetPlatformMesh))
  (bind _platformmesh_2 (Variables|Default|GetPlatformMesh))
  (bind _tiltspeed (Variables|Default|GetTiltSpeed))
  (bind _returnvalue (* _deltamultiplier DeltaSeconds))
  (bind _relativerotation (Variables|/Script/Engine.SceneComponent|GetRelativeRotation _platformmesh))
  (bind _roll (Math|Rotator|BreakRotator _relativerotation))
  ;[0.3072 0.5297 1] PlatformMesh Rotation
  (if (Variables|Default|GetIsTilting)
    (Transformation|SetRelativeRotation _platformmesh_2 (Math|Rotator|MakeRotator (Math|Interpolation|FInterpTo _roll (Variables|Default|GetTiltAngle) _returnvalue _tiltspeed) 0.0 0.0) false false)
    (else
      (Transformation|SetRelativeRotation _platformmesh_2 (Math|Rotator|MakeRotator (Math|Interpolation|FInterpTo _roll 0.0 _returnvalue _tiltspeed) 0.0 0.0) false false))))

(fn ConstructionScript)